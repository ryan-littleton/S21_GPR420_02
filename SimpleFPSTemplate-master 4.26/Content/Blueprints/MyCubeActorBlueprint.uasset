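; MyCubeActorBlueprint is an actor that grows over time at a rate set by its Price value and labels itself with RetainerName.
; Each Tick multiplies its scale by a factor slightly above one for positive Price, compounding per frame without delta-time scaling.
; Scaling and the TextRender label update only while the resulting X scale stays below a fixed cap.
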(event EventBeginPlay)

(event Collision|EventActorBeginOverlap
  (params (OtherActor :type Actor%20Object%20Reference)))

(event EventTick
  (params (DeltaSeconds :type Float%20%28single-precision%29))
  (bind _returnvalue (Transformation|GetActorScale3D))
  (bind _price (Variables|Default|GetPrice))
  (bind _returnvalue_2 (* _price 2e-06))
  (bind _returnvalue_3 (+ _returnvalue_2 1.0))
  (bind _returnvalue_4 (* _returnvalue _returnvalue_3))
  (if (< (.X (Math|Vector|BreakVector _returnvalue_4)) 7.0)
    (Transformation|SetActorScale3D _returnvalue_4)
    (Rendering|Components|TextRender|SetText (Variables|Default|GetTextRender) (Variables|Default|GetRetainerName))))

(fn ConstructionScript)