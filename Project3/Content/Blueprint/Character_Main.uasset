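; First-person player character Blueprint that handles movement, mouse look, jumping, hitscan shooting and score.
; BeginPlay creates and displays the HUD; axis inputs drive movement and sensitivity-scaled look.
; Fire, gated by a short delay, runs a debug-drawn camera line trace against PhysicsBody objects and applies damage to the hit actor.
; Overlapping the EnemyTarget actor damages the player through DamageHandler, while AddScore increments the score.
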(event EventBeginPlay
  (bind _returnvalue (UserInterface|CreateWidget "/Game/UI/HUD.HUD_C"))
  (bind _output_get (Variables|Default|SetHUD_Reference _returnvalue))
  (UserInterface|Viewport|AddtoViewport _output_get 0))

(event Collision|EventActorBeginOverlap
  (params (OtherActor :type Actor%20Object%20Reference))
  (if (== OtherActor "/Game/Blueprint/EnemyTarget.EnemyTarget")
    (Default|TakeDamage (Variables|Default|GetDamageHandler) 1.0)
    (Development|PrintString "Player taken damage")))

(event Input|ActionEvents|InputActionJump
  (params (Key :type Key%20Structure :default "None"))
  (:Pressed
    (Character|Jump)))

(event Input|ActionEvents|InputActionFire
  (params (Key :type Key%20Structure :default "None"))
  (:Pressed
    (if (Variables|Default|GetIsAbleToFire)
      (CallFunction|FireWeapon)
      (Variables|Default|SetIsAbleToFire false)
      (Utilities|FlowControl|RetriggerableDelay 0.05)
      (Variables|Default|SetIsAbleToFire true))))

(event Input|AxisEvents|InputAxisForward_Backward
  (params (AxisValue :type Float%20%28single-precision%29))
  ;[1 1 1] Basic Movement
  (Pawn|Input|AddMovementInput (Transformation|GetActorForwardVector) AxisValue false))

(event Input|AxisEvents|InputAxisStrafe_Left_Right
  (params (AxisValue :type Float%20%28single-precision%29))
  ;[1 1 1] Basic Movement
  (Pawn|Input|AddMovementInput (Transformation|GetActorRightVector) AxisValue false))

(event Input|AxisEvents|InputAxisRotate_Left_Right
  (params (AxisValue :type Float%20%28single-precision%29))
  ;[1 1 1] Mouse Look
  (Pawn|Input|AddControllerYawInput (* (Variables|Default|GetInput_Sensitivity) AxisValue)))

(event Input|AxisEvents|InputAxisLook_Up_Down
  (params (AxisValue :type Float%20%28single-precision%29))
  ;[1 1 1] Mouse Look
  (Pawn|Input|AddControllerPitchInput (* (Variables|Default|GetInput_Sensitivity) AxisValue)))

(fn ConstructionScript)

(fn FireWeapon
  (bind _camera (Variables|Default|GetCamera))
  (bind _returnvalue (Transformation|GetWorldTransform _camera))
  (bind (_location _rotation) (Math|Transform|BreakTransform _returnvalue))
  (bind (_outhit _returnvalue_2) (Collision|LineTraceForObjects _location (+ _location (* (Math|Vector|GetForwardVector _rotation) (Variables|Default|GetTraceDistance))) (Utilities|Array|MakeArray "ObjectTypeQuery4") false 0 "ForDuration"))
  (if _returnvalue_2
    (Game|Damage|ApplyDamage (.HitActor (Collision|BreakHitResult _outhit)) (Variables|Default|GetFire_Damage) 0 0)))

(fn AddScore
  (params (ScoreToAdd :type Integer))
  (Variables|Default|SetScore (+ (Variables|Default|GetScore) ScoreToAdd)))