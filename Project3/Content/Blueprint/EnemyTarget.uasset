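; EnemyTarget is a damageable enemy target actor that displays a retainer name and grows in size according to its price.
; Any damage and a custom damage event both forward to a DamageHandler.
; Tick refreshes the name text and compounds the actor's scale by a small Price-based factor until X exceeds 3.
; The overlap check against Character_Main leads to no action.
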(event Custom|CustomEvent
  (params (Damage :type Float%20%28single-precision%29) (DamageType :type Damage%20Type%20Object%20Reference) (InstigatedBy :type Controller%20Object%20Reference) (DamageCauser :type Actor%20Object%20Reference))
  (Default|TakeDamage (Variables|Default|GetDamageHandler) Damage))

(event Collision|EventActorBeginOverlap
  (params (OtherActor :type Actor%20Object%20Reference))
  (if (== OtherActor "/Game/Blueprint/Character_Main.Character_Main")
    _))

(event Game|Damage|EventAnyDamage
  (params (Damage :type Float%20%28single-precision%29) (DamageType :type Damage%20Type%20Object%20Reference) (InstigatedBy :type Controller%20Object%20Reference) (DamageCauser :type Actor%20Object%20Reference))
  (Default|TakeDamage (Variables|Default|GetDamageHandler) Damage))

(event EventTick
  (params (DeltaSeconds :type Float%20%28single-precision%29))
  (bind _returnvalue (Transformation|GetActorScale3D))
  (Rendering|Components|TextRender|SetText (Variables|Default|GetTextRender) (Variables|Default|GetRetainerName))
  (bind _output_get (Variables|Default|SetSizeV (Math|Conversions|ToVector(Float) (* (Math|Conversions|ToFloat(Integer) (Variables|Default|GetPrice)) 1e-06))))
  (if (<= (.X (Math|Vector|BreakVector _returnvalue)) 3.0)
    (Transformation|SetActorScale3D (* _returnvalue (+ _output_get 1)))))

(fn ConstructionScript)