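; DamageHandler gives its owning actor health that can be depleted by damage.
; TakeDamage subtracts the incoming damage from Health.
; When Health reaches zero or below, it spawns the P_Explosion emitter at the owner's location, rotation and scale, then destroys the owner.
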(fn TakeDamage
  (params (Damage :type Float%20%28single-precision%29))
  (bind _returnvalue (Components|GetOwner))
  (Variables|Default|SetHealth (- (Variables|Default|GetHealth) Damage))
  (if (<= (Variables|Default|GetHealth) 0.0)
    (Effects|SpawnEmitteratLocation "/Game/StarterContent/Particles/P_Explosion.P_Explosion" (Transformation|GetActorLocation _returnvalue) (Transformation|GetActorRotation _returnvalue) (Transformation|GetWorldScale (Variables|/Script/Engine.Actor|GetRootComponent _returnvalue)))
    (Actor|DestroyActor _returnvalue)))